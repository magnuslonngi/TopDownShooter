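; Base grenade actor that launches itself on spawn and explodes either after a timer or on impact.
; BeginPlay applies a velocity-change impulse to the mesh, using only the X of forward times LaunchSpeed, with LaunchAngle as raw Z.
; A nonzero TimerDelay sets a fuse, while zero makes Hit trigger the blast.
; Explode applies radial damage, spawns Niagara and sound effects at ExplotionPoint, then destroys the actor.
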(event Custom|Explode
  (bind _explotionpoint (Variables|Default|GetExplotionPoint))
  (bind _returnvalue (Transformation|GetWorldLocation _explotionpoint))
  (Game|Damage|ApplyRadialDamage 5e+01 _returnvalue 4e+02 0 0 0 0 false "ECC_Visibility")
  (Niagara|SpawnSystematLocation "/Game/Fab/MsvFx_Niagara_Explosion_Pack_01/Prefabs/Niagara_Explosion_02.Niagara_Explosion_02" _returnvalue)
  (Audio|PlaySoundatLocation "/Game/Fab/Free_Sounds_Pack/wav/Explosion_Large_1-1.Explosion_Large_1-1" _returnvalue "0, 0, 0" 1.0 1.0 0.0 0 0 0 0)
  (Actor|DestroyActor))

(event EventBeginPlay
  (bind _timerdelay (Variables|Default|GetTimerDelay))
  (Physics|AddImpulse (Variables|Default|GetMeshGrenade) (Math|Vector|MakeVector (.x (* (Transformation|GetActorForwardVector) (Variables|Default|GetLaunchSpeed))) 0.0 (Variables|Default|GetLaunchAngle)) "None" true)
  (if (!= _timerdelay 0.0)
    (Utilities|FlowControl|Delay _timerdelay)
    (CallFunction|Explode)))

(event Collision|EventActorBeginOverlap
  (params (OtherActor :type Actor%20Object%20Reference)))

(event EventTick
  (params (DeltaSeconds :type Float%20%28single-precision%29)))

(event Collision|EventHit
  (params (MyComp :type Primitive%20Component%20Object%20Reference) (Other :type Actor%20Object%20Reference) (OtherComp :type Primitive%20Component%20Object%20Reference) (bSelfMoved :type Boolean) (HitLocation :type Vector :default "0, 0, 0") (HitNormal :type Vector :default "0, 0, 0") (NormalImpulse :type Vector :default "0, 0, 0") (Hit :type Hit%20Result%20Structure%20%28by%20ref%29))
  (if (== (Variables|Default|GetTimerDelay) 0.0)
    (CallFunction|Explode)))

(fn ConstructionScript)