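; Base Blueprint for grenade pickups, which displays a spinning pickup in the world.
; On BeginPlay it resets the actor's rotation and gives the RotationPivot a random starting yaw.
; A looping timer, rather than Tick, then advances the pivot's yaw by RotationSpeed on each step.
; Interaction and range events only forward to the parent class, and the construction script is empty.
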(event Custom|RotateMeshOverTime
  (Transformation|SetRelativeRotation (Variables|Default|GetRotationPivot) (Math|Rotator|MakeRotator 0.0 0.0 (+ (.yaw (Variables|/Script/Engine.SceneComponent|GetRelativeRotation (Variables|Default|GetRotationPivot))) (Variables|InteractableData|GetRotationSpeed))) false false))

(event EventOnInteractOutOfRange
  (params (Interactor :type Actor%20Object%20Reference))
  (|CallParentFunction Interactor))

(event EventOnInteractinRange
  (params (Interactor :type Actor%20Object%20Reference))
  (|CallParentFunction Interactor))

(event EventOnInteract
  (params (Interactor :type Actor%20Object%20Reference))
  (|CallParentFunction Interactor))

(event EventBeginPlay
  (|CallParentFunction)
  (Transformation|SetActorRotation "0, 0, 0")
  (Transformation|SetRelativeRotation (Variables|Default|GetRotationPivot) (Math|Rotator|MakeRotator 0.0 0.0 (Math|Random|RandomFloatinRange 0.0 3.6e+02)) false false)
  (Utilities|Time|SetTimerbyEvent (delegate Custom|RotateMeshOverTime) 0.05 true))

(fn ConstructionScript)