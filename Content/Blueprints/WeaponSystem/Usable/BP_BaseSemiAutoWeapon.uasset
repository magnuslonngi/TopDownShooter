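; Base semi-automatic weapon Blueprint in the usable weapon system that adds a fire-rate limit to the parent's shooting.
; The Shoot override always calls the parent first, then creates a shoot trace only while CanShoot is true.
; Each shot clears that flag and starts a timer of FireRate length, which calls ResetShoot to allow firing again.
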(event Custom|ResetShoot
  ;[0.15 0.15 0.15 0.5] Overrides parent shoot to have a fire rate
  (Variables|Default|SetCanShoot? true))

(event EventShoot
  ;[0.15 0.15 0.15 0.5] Overrides parent shoot to have a fire rate
  (|CallParentFunction)
  (if (Variables|Default|GetCanShoot?)
    (Variables|Default|SetCanShoot? false)
    (CallFunction|CreateShootTrace)
    (Utilities|Time|SetTimerbyEvent (delegate Custom|ResetShoot) (Variables|Default|GetFireRate))))

(fn ConstructionScript
  (|CallParentFunction))