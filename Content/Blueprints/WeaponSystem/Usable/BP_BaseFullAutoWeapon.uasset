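; BP_BaseFullAutoWeapon is a base Blueprint for full-auto weapons that fire repeatedly until shooting ends.
; It overrides Shoot to call the parent, fire a trace immediately and start a looping timer at FireRate, which is used as the interval between traces.
; Each timer tick calls CreateShootTrace, and EndShoot calls the parent, then clears and invalidates the timer if its handle is valid.
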(event Custom|ResetShoot
  ;[0.15 0.15 0.15 0.5] Overrides parent shoot to have a fire rate
  (CallFunction|CreateShootTrace))

(event EventEndShoot
  ;[0.15 0.15 0.15 0.5] Overrides parent shoot to have a fire rate
  (|CallParentFunction)
  (if (Utilities|Time|IsValidTimerHandle (Variables|Default|GetShootTimer))
    (Utilities|Time|ClearandInvalidateTimerbyHandle (Variables|Default|GetShootTimer))))

(event EventShoot
  ;[0.15 0.15 0.15 0.5] Overrides parent shoot to have a fire rate
  (|CallParentFunction)
  (CallFunction|CreateShootTrace)
  (bind _returnvalue (Utilities|Time|SetTimerbyEvent (delegate Custom|ResetShoot) (Variables|Default|GetFireRate) true))
  (Variables|Default|SetShootTimer _returnvalue))

(fn ConstructionScript
  (|CallParentFunction))