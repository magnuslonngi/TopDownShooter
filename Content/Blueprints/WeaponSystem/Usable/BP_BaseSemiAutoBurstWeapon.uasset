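; BP_BaseSemiAutoBurstWeapon is a base semi-auto burst weapon that overrides the parent's Shoot to add a fire rate.
; Shoot always calls the parent, then, if CanShoot is set, clears it and starts a looping ShotInterval timer.
; Each tick fires a shoot trace until ShotsFired reaches ShotsPerBurst.
; The following tick clears the timer, waits out CooldownAfterBurst, then re-enables shooting and resets the count.
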(event Custom|ResetShoot
  ;[0.15 0.15 0.15 0.5] Overrides parent shoot to have a fire rate
  (if (< (Variables|Default|GetShotsFired) (Variables|Default|GetShotsPerBurst))
    (CallFunction|CreateShootTrace)
    (Math|Integer|IncrementInt (Variables|Default|GetShotsFired))
    (elif (Utilities|Time|IsValidTimerHandle (Variables|Default|GetShootIntervalTimer))
      (Utilities|Time|ClearandInvalidateTimerbyHandle (Variables|Default|GetShootIntervalTimer))
      (Utilities|FlowControl|Delay (Variables|Default|GetCooldownAfterBurst))
      (Variables|Default|SetCanShoot? true)
      (Variables|Default|SetShotsFired 0))))

(event EventShoot
  ;[0.15 0.15 0.15 0.5] Overrides parent shoot to have a fire rate
  (|CallParentFunction)
  (if (Variables|Default|GetCanShoot?)
    (Variables|Default|SetCanShoot? false)
    (bind _returnvalue (Utilities|Time|SetTimerbyEvent (delegate Custom|ResetShoot) (Variables|Default|GetShotInterval) true))
    (Variables|Default|SetShootIntervalTimer _returnvalue)))

(fn ConstructionScript
  (|CallParentFunction))