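; Base weapon Blueprint that provides hitscan firing, ammo tracking and reload logic, with Shoot and EndShoot left for children to override.
; CreateShootTrace spends a round, line-traces for pawns and static world, applies damage, and plays audio and Niagara muzzle, beam and impact effects.
; An empty magazine or owner check fires OnAmmoReload, leaving the owner to call Reload after its montage.
; Ammo data comes from pickups, and OnAmmoChange broadcasts updated counts.
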(event Custom|CreateShootTrace
  (bind _shoottracestart (Variables|Default|GetShootTraceStart))
  (bind _emptyshotaudio (Variables|Default|GetEmptyShotAudio))
  (bind _ammodata (Variables|Ammo|GetAmmoData))
  (bind _ammodata_2 (Variables|Ammo|GetAmmoData))
  (bind _ammodata_3 (Variables|Ammo|GetAmmoData))
  (bind _returnvalue (Transformation|GetWorldLocation _shoottracestart))
  ;[0.15 0.15 0.15 0.5] Creates the shoot trace, used after shoot is called on children override
  (if (> (.currentmagazineammo _ammodata_2) 0)
    (|SetBy-RefVar (Variables|Ammo|GetAmmoData) (Utilities|Struct|MakeE_AmmoData (.maxmagazineammo _ammodata_3) (- (.currentmagazineammo _ammodata_3) 1) (.maxreserveammo _ammodata_3) (.currentreserveammo _ammodata_3)))
    (Default|CallOnAmmoChange (Variables|WeaponData|GetWeaponEquipType) (.currentmagazineammo _ammodata) (.currentreserveammo _ammodata))
    (bind _output_get (Variables|ShotData|SetTraceEnd (+ _returnvalue (* (Math|Vector|GetForwardVector (Transformation|GetWorldRotation _shoottracestart)) (Variables|ShotData|GetDistance)))))
    (bind (_outhit _returnvalue_2) (Collision|LineTraceForObjects _returnvalue _output_get (Utilities|Array|MakeArray "ObjectTypeQuery3" "ObjectTypeQuery1") false 0 "None"))
    (CallFunction|SpawnTraceSystem (Transformation|GetWorldLocation (Variables|Default|GetShootTraceStart)) (.Location (Collision|BreakHitResult _outhit)) _returnvalue_2)
    (Audio|Components|Audio|Play (Variables|Default|GetShotAudio) 0.0)
    (Game|Damage|ApplyDamage (.HitActor (Collision|BreakHitResult _outhit)) (Variables|ShotData|GetDamage) 0 0)
    (elif (> (.currentreserveammo _ammodata_2) 0)
      (Audio|Components|Audio|Play _emptyshotaudio 0.0)
      (CallFunction|EndShoot)
      (Default|CallOnAmmoReload)
      (else
        (Audio|Components|Audio|Play _emptyshotaudio 0.0)))))

(event Custom|Shoot
  ;[0.15 0.15 0.15 0.5] Override on childrens
)

(event Custom|EndShoot
  ;[0.15 0.15 0.15 0.5] Override on childrens
)

(event Custom|Reload
  (bind _ammodata (Variables|Ammo|GetAmmoData))
  (bind _ammodata_2 (Variables|Ammo|GetAmmoData))
  (bind _ammodata_3 (Variables|Ammo|GetAmmoData))
  (bind _ammodata_4 (Variables|Ammo|GetAmmoData))
  ;[0.15 0.15 0.15 0.5] Event dispatcher "On Ammo Reload" has the weapon owner function to trigger the reload after montage ends
  (bind _output_get (Variables|Ammo|SetReloadAmmoNeeded (- (.maxmagazineammo _ammodata_4) (.currentmagazineammo _ammodata_4))))
  (if (>= (.currentreserveammo (Variables|Ammo|GetAmmoData)) _output_get)
    (|SetBy-RefVar (Variables|Ammo|GetAmmoData) (Utilities|Struct|MakeE_AmmoData (.maxmagazineammo _ammodata_2) (+ (.currentmagazineammo _ammodata_2) (Variables|Ammo|GetReloadAmmoNeeded)) (.maxreserveammo _ammodata_2) (- (.currentreserveammo _ammodata_2) (Variables|Ammo|GetReloadAmmoNeeded))))
    (else
      (|SetBy-RefVar (Variables|Ammo|GetAmmoData) (Utilities|Struct|MakeE_AmmoData (.maxmagazineammo _ammodata_3) (+ (.currentmagazineammo _ammodata_3) (.currentreserveammo _ammodata_3)) (.maxreserveammo _ammodata_3) 0))))
  (Default|CallOnAmmoChange (Variables|WeaponData|GetWeaponEquipType) (.currentmagazineammo _ammodata) (.currentreserveammo _ammodata)))

(event Custom|CheckForReload
  (bind _ammodata (Variables|Ammo|GetAmmoData))
  ;[0.15 0.15 0.15 0.5] Called from weapon owner, checks if the weapon needs to reload
  (if (and (> (.maxmagazineammo _ammodata) (.currentmagazineammo _ammodata)) (> (.currentreserveammo _ammodata) 0))
    (CallFunction|EndShoot)
    (Default|CallOnAmmoReload)))

(event Custom|UnbindEventDispatchers
  ;[0.15 0.15 0.15 0.5] Unbind events from character when drop/swap weapon
  (EventDispatchers|UnbindallEventsfromOnAmmoChange)
  (EventDispatchers|UnbindallEventsfromOnAmmoReload))

(event Custom|InitializeFromWeaponPickup
  (params (AmmoData :type E%20Ammo%20Data%20Structure))
  ;[0.15 0.15 0.15 0.5] Initialize weapon ammo data from the pickup
  (|SetBy-RefVar (Variables|Ammo|GetAmmoData) AmmoData))

(fn ConstructionScript)

(fn SpawnTraceSystem
  (params (StartPos :type Vector) (HitPos :type Vector) (TraceHit? :type Boolean))
  (LocalVariables|SetStartPosition StartPos)
  (LocalVariables|SetHitPosition HitPos)
  (LocalVariables|SetHit? TraceHit?)
  (Niagara|SpawnSystemAttached "/Game/VFX/NS_MuzzleFlash.NS_MuzzleFlash" (Variables|Default|GetShootTraceStart) "None" "0, 0, 0" "0.000000,-90.000000,0.000000" "KeepRelativeOffset" true)
  (bind _returnvalue (Niagara|SpawnSystematLocation "/Game/VFX/NS_TraceBeam.NS_TraceBeam" (Variables|ShotData|GetTraceEnd)))
  (bind _output_get (LocalVariables|SetParticles _returnvalue))
  (Class|NiagaraComponent|SetVariablePosition _output_get "start" (LocalVariables|GetStartPosition))
  (if (LocalVariables|GetHit?)
    (Class|NiagaraComponent|SetVariablePosition (LocalVariables|GetParticles) "end" (LocalVariables|GetHitPosition))
    (Niagara|SpawnSystematLocation "/Game/VFX/NS_MuzzleFlash.NS_MuzzleFlash" (LocalVariables|GetHitPosition) (Math|Rotator|MakeRotator (.Roll (Math|Rotator|BreakRotator (Math|Rotator|FindLookatRotation (LocalVariables|GetStartPosition) (LocalVariables|GetHitPosition)))) (.Pitch (Math|Rotator|BreakRotator (Math|Rotator|FindLookatRotation (LocalVariables|GetStartPosition) (LocalVariables|GetHitPosition)))) (+ (.Yaw (Math|Rotator|BreakRotator (Math|Rotator|FindLookatRotation (LocalVariables|GetStartPosition) (LocalVariables|GetHitPosition)))) 9e+01)))
    (else
      (Class|NiagaraComponent|SetVariablePosition (LocalVariables|GetParticles) "end" (Variables|ShotData|GetTraceEnd)))))