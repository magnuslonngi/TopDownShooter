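; Base weapon pickup actor that gives its configured weapon to whoever interacts with it.
; It extends a parent's interaction events, passing the Weapon variable to the interactor through OnWeaponSpawn and then destroying itself.
; On BeginPlay it resets its world rotation to zero, and the in-range and out-of-range events only call the parent implementation.
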(event EventOnInteractOutOfRange
  (params (Interactor :type Actor%20Object%20Reference))
  (|CallParentFunction 0))

(event EventOnInteractinRange
  (params (Interactor :type Actor%20Object%20Reference))
  (|CallParentFunction 0))

(event EventOnInteract
  (params (Interactor :type Actor%20Object%20Reference))
  (|CallParentFunction Interactor)
  (Class|BPIWeaponHolder|OnWeaponSpawn(Message) Interactor (Variables|Default|GetWeapon))
  (Actor|DestroyActor))

(event EventBeginPlay
  (|CallParentFunction)
  (Transformation|SetActorRotation "0, 0, 0"))

(fn ConstructionScript)