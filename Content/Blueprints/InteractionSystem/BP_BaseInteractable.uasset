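; Base interactable actor that displays an interaction prompt through its MessageDisplayWidget component.
; On BeginPlay it creates the InteractWidget, fills it with InteractText, resets the actor's rotation to zero and hides the prompt.
; The OnInteractinRange and OnInteractOutOfRange events show and hide the prompt; the range detection that triggers them is not part of this graph.
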(event EventBeginPlay
  (bind _returnvalue (UserInterface|CreateWidget (Variables|Default|GetInteractWidget)))
  (UserInterface|SetWidget (Variables|Default|GetMessageDisplayWidget) _returnvalue)
  (Default|SetInteractText _returnvalue (Variables|Default|GetInteractText))
  (Transformation|SetActorRotation "0, 0, 0")
  (Development|SetHiddeninGame (Variables|Default|GetMessageDisplayWidget) true false))

(event EventOnInteractinRange
  (params (Interactor :type Actor%20Object%20Reference))
  (Development|SetHiddeninGame (Variables|Default|GetMessageDisplayWidget) false false))

(event EventOnInteractOutOfRange
  (params (Interactor :type Actor%20Object%20Reference))
  (Development|SetHiddeninGame (Variables|Default|GetMessageDisplayWidget) true false))

(fn ConstructionScript)