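; Base enemy character that melees the player and dies when its health runs out.
; BeginPlay loads health and walk speed from a DT_EnemyTypes row, whose stats also drive attacks.
; Tick checks player distance, applying damage as the attack montage starts, with a Delay-gated cooldown.
; AnyDamage reduces health; death disables movement and collision, then destroys the actor after its montage, with both montages hardcoded to werewolf animations.
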(event EventBeginPlay
  (bind _returnvalue (Utilities|GetDataTableRow "/Game/Blueprints/EnemySystem/Data/DT_EnemyTypes.DT_EnemyTypes" (Variables|Default|GetRowName))
    (:then
      (Variables|Default|SetStats _returnvalue)
      (Variables|Default|SetCurrentHealth (.MaxHealth (Utilities|Struct|BreakS_EnemyStats (Variables|Default|GetStats))))
      (Variables|/Script/Engine.CharacterMovementComponent|SetMaxWalkSpeed (Variables|Character|GetCharacterMovement) (.WalkSpeed (Utilities|Struct|BreakS_EnemyStats (Variables|Default|GetStats)))))))

(event Collision|EventActorBeginOverlap
  (params (OtherActor :type Actor%20Object%20Reference)))

(event EventTick
  (params (DeltaSeconds :type Float%20%28single-precision%29))
  (bind _stats (Variables|Default|GetStats))
  (bind (_maxhealth _walkspeed _chasespeed _meleedamage _attackrange _attackcooldown) (Utilities|Struct|BreakS_EnemyStats _stats))
  (if (not (Variables|Default|GetbDead))
    (if (and (Variables|Default|GetbCanAttack) (<= (Transformation|GetDistanceTo (Game|GetPlayerCharacter 0)) _attackrange))
      (Variables|Default|SetbCanAttack false)
      (Animation|PlayAnimMontage "/Game/Animations/Wolf/AM_WerewolfAttack.AM_WerewolfAttack" 1.0 "None")
      (Game|Damage|ApplyDamage (Game|GetPlayerCharacter 0) _meleedamage (Pawn|GetController) self)
      (Utilities|FlowControl|Delay _attackcooldown)
      (Variables|Default|SetbCanAttack true))))

(event Game|Damage|EventAnyDamage
  (params (Damage :type Float%20%28single-precision%29) (DamageType :type Damage%20Type%20Object%20Reference) (InstigatedBy :type Controller%20Object%20Reference) (DamageCauser :type Actor%20Object%20Reference))
  (bind _output_get (Variables|Default|SetCurrentHealth (- (Variables|Default|GetCurrentHealth) Damage)))
  (if (and (<= _output_get 0.0) (not (Variables|Default|GetbDead)))
    (Variables|Default|SetbDead true)
    (Pawn|Components|CharacterMovement|DisableMovement (Variables|Character|GetCharacterMovement))
    (Collision|SetCollisionEnabled (Variables|Collision|GetCapsuleComponent) "NoCollision")
    (bind _returnvalue (Animation|PlayAnimMontage "/Game/Animations/Wolf/AM_WerewolfDeath.AM_WerewolfDeath" 1.0 "None"))
    (Utilities|FlowControl|Delay _returnvalue)
    (Actor|DestroyActor self)))

(fn ConstructionScript)