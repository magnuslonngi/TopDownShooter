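; Player HUD for the TDS game that owns the character widget and handles the fail and pause screens.
; It creates the character widget on BeginPlay and forwards stamina, health, ammo and grenade updates to it, routing the latter two by primary or secondary slot.
; Zero health swaps that widget for the fail menu.
; PauseGame toggles pause, input mode and cursor using a PauseMenu reference not created here; VictoryGame is empty.
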(event EventBeginPlay
  (bind _returnvalue (UserInterface|CreateWidget "/Game/Blueprints/Player/UI/BPW_Character.BPW_Character_C"))
  (bind _output_get (Variables|Default|SetCharacterWidget _returnvalue))
  (UserInterface|Viewport|AddtoViewport _output_get 0))

(event EventUpdateHealth
  (params (CurrentHealth :type Float%20%28double-precision%29) (MaxHealth :type Float%20%28double-precision%29))
  (Default|UpdateHealthBar (Variables|Default|GetCharacterWidget) CurrentHealth MaxHealth)
  (if (<= CurrentHealth 0.0)
    (Widget|RemovefromParent (Variables|Default|GetCharacterWidget))
    (bind _returnvalue (UserInterface|CreateWidget "/Game/UI/Menus/WBP_Fail_Menu.WBP_Fail_Menu_C"))
    (UserInterface|Viewport|AddtoViewport _returnvalue 0)))

(event EventUpdateAmmo
  (params (WeaponEquipType :type E_WeaponEquipType%20Enum :default "NewEnumerator0") (CurrentMagAmmo :type Integer) (CurrentAmmo :type Integer))
  (switch Utilities|FlowControl|Switch|SwitchonE_WeaponEquipType WeaponEquipType
    (:NewEnumerator0
      (Default|UpdatePrimaryAmmo (Variables|Default|GetCharacterWidget) CurrentMagAmmo CurrentAmmo))
    (:NewEnumerator1
      (Default|UpdateSecondaryAmmo (Variables|Default|GetCharacterWidget) CurrentMagAmmo CurrentAmmo))))

(event EventUpdateGrenade
  (params (GrenadeEquipType :type E_WeaponEquipType%20Enum :default "NewEnumerator0") (GrenadeCount :type Integer))
  (switch Utilities|FlowControl|Switch|SwitchonE_WeaponEquipType GrenadeEquipType
    (:NewEnumerator0
      (Default|UpdatePrimaryGrenadeCount (Variables|Default|GetCharacterWidget) GrenadeCount))
    (:NewEnumerator1
      (Default|UpdateSecondaryGrenadeCount (Variables|Default|GetCharacterWidget) GrenadeCount))))

(event EventUpdateStamina
  (params (CurrentStamina :type Float%20%28double-precision%29) (MaxStamina :type Float%20%28double-precision%29))
  (Default|UpdateStaminaBar (Variables|Default|GetCharacterWidget) CurrentStamina MaxStamina))

(event EventPauseGame
  (bind _returnvalue (Game|GetPlayerController 0))
  (bind _pausemenu (Variables|Default|GetPauseMenu))
  (if (Variables|Default|GetisPaused)
    (Game|SetGamePaused false)
    (Widget|RemovefromParent (Variables|Default|GetPauseMenu))
    (Input|SetInputModeGameOnly _returnvalue false)
    (Variables|Default|SetisPaused false)
    (Variables|/Script/Engine.PlayerController|SetbShowMouseCursor _returnvalue false)
    (else
      (Game|SetGamePaused true)
      (UserInterface|Viewport|AddtoViewport _pausemenu 0)
      (Input|SetInputModeUIOnly _returnvalue _pausemenu "DoNotLock" false)
      (Variables|Default|SetisPaused true)
      (Variables|/Script/Engine.PlayerController|SetbShowMouseCursor _returnvalue true))))

(event EventVictoryGame)

(fn ConstructionScript)