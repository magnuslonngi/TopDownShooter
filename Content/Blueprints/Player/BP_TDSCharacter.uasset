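; Top-down shooter player character that handles movement, mouse aiming, sprinting, shooting and interaction through interface events called by the controller.
; Sprinting drains stamina through self-repeating delayed events that update the HUD, with regeneration on stop and a cooldown when depleted.
; A looping timer sphere-traces for the closest interactable and sends it range messages.
; Equipping a weapon drops the current one as a pickup and attaches the new one to a mesh socket.
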(event Custom|DrainStaminaConstantly
  ;[0.15 0.15 0.15 0.5] Run logic when controller calls the interface
  (Variables|Stamina|SetStamina (Math|Float|Clamp(Float) (- (Variables|Stamina|GetStamina) (Variables|Stamina|GetRunDrainStamina)) 0.0 (Variables|Stamina|GetMaxStamina)))
  (bind _hud (Utilities|GetHUD))
  (Class|BPIPlayerHUD|UpdateStamina(Message) _hud (Variables|Stamina|GetStamina) (Variables|Stamina|GetMaxStamina))
  (if (== (Variables|Stamina|GetStamina) 0.0)
    ;;[0.15 0.15 0.15 0.5] When we hit 0 stamina, we wait for certain time to be able to run
    (CallFunction|StopRunning)
    (Variables|Default|SetCanRun? false)
    (Utilities|Time|SetTimerbyEvent (delegate Custom|EnableRunOnCooldown) (Variables|Stamina|GetRunCooldownOnDeplete))
    (else
      ;;[0.15 0.15 0.15 0.5] Repeat the function to keep draining
      (if (Variables|Default|GetIsRunning?)
        (Utilities|FlowControl|Delay 0.05)
        (CallFunction|DrainStaminaConstantly)))))

(event Custom|RegainStaminaConstantly
  ;[0.15 0.15 0.15 0.5] Run logic when controller calls the interface
  (Variables|Stamina|SetStamina (Math|Float|Clamp(Float) (+ (Variables|Stamina|GetStamina) (Variables|Stamina|GetConstantRegainStamina)) 0.0 (Variables|Stamina|GetMaxStamina)))
  (bind _hud (Utilities|GetHUD))
  (Class|BPIPlayerHUD|UpdateStamina(Message) _hud (Variables|Stamina|GetStamina) (Variables|Stamina|GetMaxStamina))
  (if (< (Variables|Stamina|GetStamina) (Variables|Stamina|GetMaxStamina))
    ;;[0.15 0.15 0.15 0.5] Repeat the funcion to keep regaining
    (if (not (Variables|Default|GetIsRunning?))
      (Utilities|FlowControl|Delay 0.05)
      (CallFunction|RegainStaminaConstantly))))

(event Custom|EnableRunOnCooldown
  ;[0.15 0.15 0.15 0.5] Run logic when controller calls the interface
  ;;[0.15 0.15 0.15 0.5] When we hit 0 stamina, we wait for certain time to be able to run
  (Variables|Default|SetCanRun? true))

(event EventOnInteractStarted
  (bind _interactableinrange (Variables|Default|GetInteractableInRange))
  ;[0.15 0.15 0.15 0.5] Interaction when controller calls the interface. Gets the interactable in range and interact.
  (Utilities|IsValid _interactableinrange
    (:Is%20Valid
      (Class|BPIInteraction|OnInteract(Message) _interactableinrange self))))

(event EventOnMouseTriggered
  (params (Location :type Vector :default "0, 0, 0"))
  (bind (_x _y _z) (Math|Vector|BreakVector Location))
  (bind _returnvalue (Transformation|GetActorLocation))
  ;[0.15 0.15 0.15 0.5] Rotates character towards the mouse location
  (Transformation|SetActorRotation (Math|Interpolation|RInterpTo (Transformation|GetActorRotation) (Math|Rotator|FindLookatRotation (Math|Vector|MakeVector (.x _returnvalue) (.y _returnvalue) _z) (Math|Vector|MakeVector _x _y _z)) (Utilities|Time|GetWorldDeltaSeconds) (Variables|Default|GetAimRotationSpeed))))

(event EventOnMoveTriggered
  (params (ActionValueX :type Float%20%28double-precision%29) (ActionValueY :type Float%20%28double-precision%29))
  (bind _returnvalue (Pawn|GetControlRotation :!class /Script/Engine.Pawn))
  ;[0.15 0.15 0.15 0.5] Moves character when controller calls the interface
  (Pawn|Input|AddMovementInput (Math|Vector|GetRightVector (Math|Rotator|MakeRotator (.roll _returnvalue) 0.0 (.yaw _returnvalue))) ActionValueX false)
  (Pawn|Input|AddMovementInput (Math|Vector|GetForwardVector (Math|Rotator|MakeRotator 0.0 0.0 (.yaw (Pawn|GetControlRotation :!class /Script/Engine.Pawn)))) ActionValueY false))

(event EventOnWeaponSpawn
  (params (Weapon :type BP%20Base%20Weapon%20Class%20Reference))
  (Utilities|IsValid (Variables|Default|GetCurrentWeapon)
    (:Is%20Valid
      (Game|SpawnActorfromClass (Variables|/Game/Blueprints/WeaponSystem/Usable/BP_BaseWeapon.BP_BaseWeapon_C|GetWeaponPickup (Variables|Default|GetCurrentWeapon)) (Transformation|GetActorTransform (Variables|Default|GetCurrentWeapon)) "Undefined" "MultiplyWithRoot" 0 0)
      (Actor|DestroyActor (Variables|Default|GetCurrentWeapon)))
    (:Is%20Not%20Valid
      _))
  (bind _returnvalue (Game|SpawnActorfromClass Weapon (Transformation|GetActorTransform) "Undefined" "MultiplyWithRoot" 0 0))
  (bind _output_get (Variables|Default|SetCurrentWeapon _returnvalue))
  (Transformation|AttachComponentToComponent _output_get (Variables|Character|GetMesh) (Variables|Default|GetWeaponSocketName) "SnapToTarget" "SnapToTarget" "SnapToTarget" true))

(event EventBeginPlay
  ;[0.15 0.15 0.15 0.5] Initialize the timer to check for interactables in range
  (Utilities|Time|SetTimerbyFunctionName 0 "CheckForInteractables" 0.1 true))

(event EventOnRunStarted
  ;[0.15 0.15 0.15 0.5] Run logic when controller calls the interface
  (CallFunction|StartRunning))

(event EventOnRunEnded
  ;[0.15 0.15 0.15 0.5] Run logic when controller calls the interface
  (CallFunction|StopRunning))

(event EventOnShootStarted
  (bind _currentweapon (Variables|Default|GetCurrentWeapon))
  (Utilities|IsValid _currentweapon
    (:Is%20Valid
      (Default|Shoot _currentweapon))))

(event EventOnShootEnded
  (bind _currentweapon (Variables|Default|GetCurrentWeapon))
  (Utilities|IsValid _currentweapon
    (:Is%20Valid
      (Default|EndShoot _currentweapon))))

(fn ConstructionScript)

(fn StartRunning
  (if (Variables|Default|GetCanRun?)
    (Variables|/Script/Engine.CharacterMovementComponent|SetMaxWalkSpeed (Variables|Character|GetCharacterMovement) 6e+02)
    (Variables|Default|SetIsRunning? true)
    (CallFunction|DrainStaminaConstantly)))

(fn StopRunning
  (Variables|/Script/Engine.CharacterMovementComponent|SetMaxWalkSpeed (Variables|Character|GetCharacterMovement) 3e+02)
  (Variables|Default|SetIsRunning? false)
  (CallFunction|RegainStaminaConstantly))

(fn CheckforInteractables
  (bind _returnvalue (Transformation|GetActorLocation))
  ;[0.15 0.15 0.15 0.5] Checks if there are interactables in range. If not, set null interactable in range.
  (bind (_outhits _returnvalue_2) (Collision|MultiSphereTraceByChannel _returnvalue _returnvalue 1e+02 "TraceTypeQuery4" false 0 "None"))
  (if _returnvalue_2
    (LocalVariables|SetClosestInteractable (.HitActor (Collision|BreakHitResult (Utilities|Array|Get(acopy) _outhits))))
    ;[0.15 0.15 0.15 0.5] Loop through each interactable in range to find the closest one and asign it to Closest Interactable global variable
    (for _array_element _outhits
      (if (< (Math|Vector|Distance(Vector) (Transformation|GetActorLocation) (Transformation|GetActorLocation (.HitActor (Collision|BreakHitResult _array_element)))) (Math|Vector|Distance(Vector) (Transformation|GetActorLocation) (Transformation|GetActorLocation (LocalVariables|GetClosestInteractable))))
        (LocalVariables|SetClosestInteractable (.HitActor (Collision|BreakHitResult _array_element)))))
    (Utilities|IsValid (Variables|Default|GetInteractableInRange)
      (:Is%20Valid
        (Class|BPIInteraction|OnInteractOutOfRange(Message) (Variables|Default|GetInteractableInRange))
        (bind _output_get (Variables|Default|SetInteractableInRange (LocalVariables|GetClosestInteractable)))
        (Class|BPIInteraction|OnInteractinRange(Message) _output_get))
      (:Is%20Not%20Valid
        (bind _output_get_2 (Variables|Default|SetInteractableInRange (LocalVariables|GetClosestInteractable)))
        (Class|BPIInteraction|OnInteractinRange(Message) _output_get_2)))
    (else
      (Utilities|IsValid (Variables|Default|GetInteractableInRange)
        (:Is%20Valid
          (Class|BPIInteraction|OnInteractOutOfRange(Message) (Variables|Default|GetInteractableInRange))
          (Variables|Default|SetInteractableInRange 0))))))

(fn GetEquipedWeponHoldType
  (bind _currentweapon (Variables|Default|GetCurrentWeapon))
  (Utilities|IsValid _currentweapon
    (:Is%20Valid
      (return (Variables|/Game/Blueprints/WeaponSystem/Usable/BP_BaseWeapon.BP_BaseWeapon_C|GetWeaponHoldType _currentweapon)))
    (:Is%20Not%20Valid
      (return "NewEnumerator4"))))